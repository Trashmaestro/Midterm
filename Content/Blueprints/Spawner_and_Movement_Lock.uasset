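; A checkpoint actor for a side-scroller that respawns the player when they stop or stop moving toward negative Y.
; Player overlap stores this actor as the character's BOX and arms the velocity check on Tick.
; A failed check spawns a fresh SideScrollerCharacter at BOX, copies the reference, destroys the old pawn and possesses the new one.
; The Respawn function repeats that sequence on a boolean input, with both guarded by DoOnce.
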(event EventTick
  (params (DeltaSeconds :type Float%20%28single-precision%29))
  (bind _returnvalue (Game|GetPlayerCharacter 0))
  (bind _asside_scroller_character (Utilities|Casting|CastToSideScrollerCharacter _returnvalue))
  (if (and (< -0.5 (.y (Transformation|GetVelocity (Game|GetPlayerCharacter 0)))) (stale Collision|EventActorBeginOverlap _output_get))
    (Utilities|FlowControl|DoOnce true :!label _label
      (:Completed
        (bind _returnvalue_2 (Game|SpawnActorfromClass "/Game/SideScrollerBP/Blueprints/SideScrollerCharacter.SideScrollerCharacter_C" (Math|Transform|MakeTransform (Transformation|GetWorldLocation (Variables|/Script/Engine.Actor|GetRootComponent (Variables|/Game/SideScrollerBP/Blueprints/SideScrollerCharacter.SideScrollerCharacter_C|GetBOX _asside_scroller_character))) "0,-90.000000, 0" "1,1,1") "Undefined" 0 0))
        (Variables|/Game/SideScrollerBP/Blueprints/SideScrollerCharacter.SideScrollerCharacter_C|SetBOX _returnvalue_2 (Variables|/Game/SideScrollerBP/Blueprints/SideScrollerCharacter.SideScrollerCharacter_C|GetBOX _asside_scroller_character))
        (Actor|DestroyActor _returnvalue)
        (Pawn|Possess (Game|GetPlayerController 0) _returnvalue_2)
        (goto _label Reset)))))

(event Collision|EventActorBeginOverlap
  (params (OtherActor :type Actor%20Object%20Reference))
  (bind _returnvalue (Game|GetPlayerCharacter 0))
  (if (== _returnvalue OtherActor)
    (bind _asside_scroller_character (Utilities|Casting|CastToSideScrollerCharacter _returnvalue))
    (Variables|/Game/SideScrollerBP/Blueprints/SideScrollerCharacter.SideScrollerCharacter_C|SetBOX _asside_scroller_character self)
    (bind _output_get (Variables|Default|SetIsPlayerRunning true))
    (Utilities|FlowControl|Delay 2.0)
    (Utilities|FlowControl|DoOnce true) ; enters at Reset
  ))

(fn ConstructionScript)

(fn Respawn
  (params (Guh :type Boolean))
  (bind _returnvalue (Game|GetPlayerCharacter 0))
  (bind _asside_scroller_character (Utilities|Casting|CastToSideScrollerCharacter _returnvalue))
  (if Guh
    (Utilities|FlowControl|DoOnce true :!label _label
      (:Completed
        (bind _returnvalue_2 (Game|SpawnActorfromClass "/Game/SideScrollerBP/Blueprints/SideScrollerCharacter.SideScrollerCharacter_C" (Math|Transform|MakeTransform (Transformation|GetActorLocation (Variables|/Game/SideScrollerBP/Blueprints/SideScrollerCharacter.SideScrollerCharacter_C|GetBOX _asside_scroller_character)) "0,-90.000000, 0" "1,1,1") "Undefined" 0 0))
        (Variables|/Game/SideScrollerBP/Blueprints/SideScrollerCharacter.SideScrollerCharacter_C|SetBOX _returnvalue_2 (Variables|/Game/SideScrollerBP/Blueprints/SideScrollerCharacter.SideScrollerCharacter_C|GetBOX _asside_scroller_character))
        (Actor|DestroyActor _returnvalue)
        (Pawn|Possess (Game|GetPlayerController 0) _returnvalue_2)
        (goto _label Reset)))))